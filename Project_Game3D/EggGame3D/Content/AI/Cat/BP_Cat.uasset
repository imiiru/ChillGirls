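; Cat AI pawn that wanders the navmesh and moves toward pawns it sees.
; From BeginPlay, RandomRoam moves to random nearby reachable points, repeating after a short pause only on success.
; PawnSensing sightings start a move to the seen pawn, and a retriggerable delay resumes roaming one second after the last sighting.
; Walk speed is set to the same value when chasing and when resuming roam.
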(event OnSeePawn(PawnSensing)
  (params (Pawn :type Pawn%20Object%20Reference))
  (Variables|/Script/Engine.CharacterMovementComponent|SetMaxWalkSpeed (Variables|Character|GetCharacterMovement) 4e+02)
  (AI|AIMoveTo self "0, 0, 0" Pawn 5.0 false
    (:then
      (Utilities|FlowControl|RetriggerableDelay 1.0)
      (Variables|/Script/Engine.CharacterMovementComponent|SetMaxWalkSpeed (Variables|Character|GetCharacterMovement) 4e+02)
      (CallFunction|RandomRoam))))

(event Custom|RandomRoam
  (bind _randomlocation (Class|NavigationSystemV1|GetRandomLocationinNavigableRadius (Transformation|GetActorLocation) 1e+03 0 0))
  (AI|AIMoveTo self _randomlocation 0 5.0 false
    (:OnSuccess
      (Utilities|FlowControl|Delay 1.0)
      (CallFunction|RandomRoam))))

(event EventBeginPlay
  (CallFunction|RandomRoam))

(event Collision|EventActorBeginOverlap
  (params (OtherActor :type Actor%20Object%20Reference)))

(event EventTick
  (params (DeltaSeconds :type Float%20%28single-precision%29)))

(fn ConstructionScript)